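; Steering-behavior agent that drives a physics cone to seek, flee from or arrive at the first BP_Target actor found at BeginPlay.
; Each tick, the AgentType setting picks the behavior, which steers the current velocity toward a desired velocity using a force capped at MaxForce.
; Seek and Flee hold MaxVel, while Arrive scales speed down with remaining distance once inside that range.
; The velocity drives the cone's physics and facing, with debug lines showing each vector.
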(event EventBeginPlay
  (bind _output_get (Variables|Default|SetCurrentVel "-1000.000000,1000.000000,10.000000"))
  (Physics|SetPhysicsLinearVelocity (Variables|Default|GetCone) (* (Math|Vector|Normalize _output_get) (Variables|Default|GetMaxVel)) false "None")
  (bind _returnvalue (Actor|GetActorOfClass "/Game/Steerings/BP_Target.BP_Target_C"))
  (Variables|Default|SetTarget _returnvalue))

(event Collision|EventActorBeginOverlap
  (params (OtherActor :type Actor%20Object%20Reference)))

(event EventTick
  (params (DeltaSeconds :type Float%20%28single-precision%29))
  (bind _target (Variables|Default|GetTarget))
  (bind _defaultsceneroot (Variables|/Game/Steerings/BP_Target.BP_Target_C|GetDefaultSceneRoot _target))
  (bind _returnvalue (Transformation|GetWorldLocation _defaultsceneroot))
  (switch Utilities|FlowControl|Switch|SwitchonSteeringType (Variables|Default|GetAgentType)
    (:NewEnumerator0
      (CallFunction|Seek _returnvalue true))
    (:NewEnumerator1
      (CallFunction|Flee _returnvalue true))
    (:NewEnumerator2
      (CallFunction|Arrive _returnvalue true)))
  (Physics|SetPhysicsLinearVelocity (Variables|Default|GetCone) (Variables|Default|GetCurrentVel) false "None")
  (CallFunction|LookatDirection))

(fn ConstructionScript)

(fn Seek
  (params (Pos :type Vector) (Debug :type Boolean))
  (bind _cone (Variables|Default|GetCone))
  (bind _cone_2 (Variables|Default|GetCone))
  (bind _relativelocation (Variables|/Script/Engine.SceneComponent|GetRelativeLocation _cone))
  (bind _relativelocation_2 (Variables|/Script/Engine.SceneComponent|GetRelativeLocation _cone_2))
  (LocalVariables|SetTargetPos Pos)
  (LocalVariables|Set_Debug Debug)
  (Utilities|FlowControl|Sequence
    (:then_0
      ;[0.03415 1 0] CreateDesiredVel
      (Variables|Default|SetDesiredVel (* (Math|Vector|Normalize (- (LocalVariables|GetTargetPos) (Variables|/Script/Engine.SceneComponent|GetRelativeLocation (Variables|Default|GetCone)))) (Variables|Default|GetMaxVel))))
    (:then_1
      ;[1 0.7805 0.09399] Debug DesiredVel
      (if (LocalVariables|Get_Debug)
        (Rendering|Debug|DrawDebugLine _relativelocation_2 (+ _relativelocation_2 (Variables|Default|GetDesiredVel)) "(R=1.000000,G=0.413427,B=0.000000,A=1.000000)" 0.0 1e+01)))
    (:then_2
      ;[0.03266 1 0] SteeringVel
      (LocalVariables|SetResta (- (Variables|Default|GetDesiredVel) (Variables|Default|GetCurrentVel)))
      (if (> (Math|Vector|VectorLength (LocalVariables|GetResta)) (Math|Vector|VectorLength (* (Math|Vector|Normalize (LocalVariables|GetResta)) (Variables|Default|GetMaxForce))))
        (Variables|Default|SetSteeringForce (* (Math|Vector|Normalize (LocalVariables|GetResta)) (Variables|Default|GetMaxForce)))
        (else
          (Variables|Default|SetSteeringForce (LocalVariables|GetResta)))))
    (:then_3
      ;[1 0.8048 0.07855] Steering
      (if (LocalVariables|Get_Debug)
        (Rendering|Debug|DrawDebugLine (+ (Variables|/Script/Engine.SceneComponent|GetRelativeLocation (Variables|Default|GetCone)) (Variables|Default|GetCurrentVel)) (+ (+ (Variables|/Script/Engine.SceneComponent|GetRelativeLocation (Variables|Default|GetCone)) (Variables|Default|GetCurrentVel)) (Variables|Default|GetSteeringForce)) "(R=0.091253,G=1.000000,B=0.000000,A=1.000000)" 0.0 1e+01)))
    (:then_4
      ;[0 1 0.04714] Add Steering to Current
      (Variables|Default|SetCurrentVel (* (Math|Vector|Normalize (+ (Variables|Default|GetCurrentVel) (Variables|Default|GetSteeringForce))) (Variables|Default|GetMaxVel))))
    (:then_5
      ;[0.9011 1 0.1274] Debug CurrentVel
      (if (LocalVariables|Get_Debug)
        (Rendering|Debug|DrawDebugLine _relativelocation (+ _relativelocation (Variables|Default|GetCurrentVel)) "(R=0.000000,G=0.098495,B=1.000000,A=1.000000)" 0.0 0.0)))))

(fn LookatDirection
  (bind _cone (Variables|Default|GetCone))
  (bind _currentvel (Variables|Default|GetCurrentVel))
  (bind _cone_2 (Variables|Default|GetCone))
  (bind _returnvalue (Transformation|GetWorldLocation _cone_2))
  (bind _relativelocation (Variables|/Script/Engine.SceneComponent|GetRelativeLocation _cone))
  (bind _returnvalue_2 (+ _relativelocation _currentvel))
  (bind _returnvalue_3 (Math|Rotator|FindLookatRotation _returnvalue _returnvalue_2))
  (bind (_roll _pitch _yaw) (Math|Rotator|BreakRotator _returnvalue_3))
  (Transformation|SetWorldRotation (Variables|Default|GetCone) (Math|Rotator|MakeRotator _roll (+ _pitch -9e+01) _yaw) false false))

(fn Flee
  (params (Pos :type Vector) (Debug :type Boolean))
  (bind _cone (Variables|Default|GetCone))
  (bind _cone_2 (Variables|Default|GetCone))
  (bind _relativelocation (Variables|/Script/Engine.SceneComponent|GetRelativeLocation _cone))
  (bind _relativelocation_2 (Variables|/Script/Engine.SceneComponent|GetRelativeLocation _cone_2))
  (LocalVariables|SetTargetPos Pos)
  (LocalVariables|Set_Debug Debug)
  (Utilities|FlowControl|Sequence
    (:then_0
      ;[0.03415 1 0] CreateDesiredVel
      (Variables|Default|SetDesiredVel (* (Math|Vector|Normalize (- (Variables|/Script/Engine.SceneComponent|GetRelativeLocation (Variables|Default|GetCone)) (LocalVariables|GetTargetPos))) (Variables|Default|GetMaxVel))))
    (:then_1
      ;[1 0.7805 0.09399] Debug DesiredVel
      (if (LocalVariables|Get_Debug)
        (Rendering|Debug|DrawDebugLine _relativelocation_2 (+ _relativelocation_2 (Variables|Default|GetDesiredVel)) "(R=1.000000,G=0.413427,B=0.000000,A=1.000000)" 0.0 1e+01)))
    (:then_2
      ;[0.03266 1 0] SteeringVel
      (LocalVariables|SetResta (- (Variables|Default|GetDesiredVel) (Variables|Default|GetCurrentVel)))
      (if (> (Math|Vector|VectorLength (LocalVariables|GetResta)) (Math|Vector|VectorLength (* (Math|Vector|Normalize (LocalVariables|GetResta)) (Variables|Default|GetMaxForce))))
        (Variables|Default|SetSteeringForce (* (Math|Vector|Normalize (LocalVariables|GetResta)) (Variables|Default|GetMaxForce)))
        (else
          (Variables|Default|SetSteeringForce (LocalVariables|GetResta)))))
    (:then_3
      ;[1 0.8048 0.07855] Steering
      (if (LocalVariables|Get_Debug)
        (Rendering|Debug|DrawDebugLine (+ (Variables|/Script/Engine.SceneComponent|GetRelativeLocation (Variables|Default|GetCone)) (Variables|Default|GetCurrentVel)) (+ (+ (Variables|/Script/Engine.SceneComponent|GetRelativeLocation (Variables|Default|GetCone)) (Variables|Default|GetCurrentVel)) (Variables|Default|GetSteeringForce)) "(R=0.091253,G=1.000000,B=0.000000,A=1.000000)" 0.0 1e+01)))
    (:then_4
      ;[0 1 0.04714] Add Steering to Current
      (Variables|Default|SetCurrentVel (* (Math|Vector|Normalize (+ (Variables|Default|GetCurrentVel) (Variables|Default|GetSteeringForce))) (Variables|Default|GetMaxVel))))
    (:then_5
      ;[0.9011 1 0.1274] Debug CurrentVel
      (if (LocalVariables|Get_Debug)
        (Rendering|Debug|DrawDebugLine _relativelocation (+ _relativelocation (Variables|Default|GetCurrentVel)) "(R=0.000000,G=0.098495,B=1.000000,A=1.000000)" 0.0 0.0)))))

(fn Arrive
  (params (Pos :type Vector) (Debug :type Boolean))
  (bind _cone (Variables|Default|GetCone))
  (bind _cone_2 (Variables|Default|GetCone))
  (bind _relativelocation (Variables|/Script/Engine.SceneComponent|GetRelativeLocation _cone))
  (bind _relativelocation_2 (Variables|/Script/Engine.SceneComponent|GetRelativeLocation _cone_2))
  (LocalVariables|SetTargetPos Pos)
  (LocalVariables|Set_Debug Debug)
  (Utilities|FlowControl|Sequence
    (:then_0
      ;[0.03415 1 0] CreateDesiredVel
      (bind _output_get (LocalVariables|SetRestaDesired (- (LocalVariables|GetTargetPos) (Variables|/Script/Engine.SceneComponent|GetRelativeLocation (Variables|Default|GetCone)))))
      (bind _output_get_2 (LocalVariables|SetDesiredLenght (Math|Vector|VectorLength _output_get)))
      (if (< _output_get_2 (Math|Vector|VectorLength (* (Math|Vector|Normalize (- (LocalVariables|GetTargetPos) (Variables|/Script/Engine.SceneComponent|GetRelativeLocation (Variables|Default|GetCone)))) (Variables|Default|GetMaxVel))))
        (Variables|Default|SetDesiredVel (LocalVariables|GetRestaDesired))
        (LocalVariables|SetArriving true)
        (else
          (Variables|Default|SetDesiredVel (* (Math|Vector|Normalize (- (LocalVariables|GetTargetPos) (Variables|/Script/Engine.SceneComponent|GetRelativeLocation (Variables|Default|GetCone)))) (Variables|Default|GetMaxVel)))
          (LocalVariables|SetArriving false))))
    (:then_1
      ;[1 0.7805 0.09399] Debug DesiredVel
      (if (LocalVariables|Get_Debug)
        (Rendering|Debug|DrawDebugLine _relativelocation_2 (+ _relativelocation_2 (Variables|Default|GetDesiredVel)) "(R=1.000000,G=0.413427,B=0.000000,A=1.000000)" 0.0 1e+01)))
    (:then_2
      ;[0.03266 1 0] SteeringVel
      (LocalVariables|SetRestaSteering (- (Variables|Default|GetDesiredVel) (Variables|Default|GetCurrentVel)))
      (if (> (Math|Vector|VectorLength (LocalVariables|GetRestaSteering)) (Math|Vector|VectorLength (* (Math|Vector|Normalize (LocalVariables|GetRestaSteering)) (Variables|Default|GetMaxForce))))
        (Variables|Default|SetSteeringForce (* (Math|Vector|Normalize (LocalVariables|GetRestaSteering)) (Variables|Default|GetMaxForce)))
        (else
          (Variables|Default|SetSteeringForce (LocalVariables|GetRestaSteering)))))
    (:then_3
      ;[1 0.8048 0.07855] Steering
      (if (LocalVariables|Get_Debug)
        (Rendering|Debug|DrawDebugLine (+ (Variables|/Script/Engine.SceneComponent|GetRelativeLocation (Variables|Default|GetCone)) (Variables|Default|GetCurrentVel)) (+ (+ (Variables|/Script/Engine.SceneComponent|GetRelativeLocation (Variables|Default|GetCone)) (Variables|Default|GetCurrentVel)) (Variables|Default|GetSteeringForce)) "(R=0.091253,G=1.000000,B=0.000000,A=1.000000)" 0.0 1e+01)))
    (:then_4
      ;[0 1 0.04714] Add Steering to Current
      (if (LocalVariables|GetArriving)
        (Variables|Default|SetCurrentVel (* (Math|Vector|Normalize (+ (Variables|Default|GetDesiredVel) (Variables|Default|GetSteeringForce))) (LocalVariables|GetDesiredLenght)))
        (else
          (Variables|Default|SetCurrentVel (* (Math|Vector|Normalize (+ (Variables|Default|GetCurrentVel) (Variables|Default|GetSteeringForce))) (Variables|Default|GetMaxVel))))))
    (:then_5
      ;[0.9011 1 0.1274] Debug CurrentVel
      (if (LocalVariables|Get_Debug)
        (Rendering|Debug|DrawDebugLine _relativelocation (+ _relativelocation (Variables|Default|GetCurrentVel)) "(R=0.000000,G=0.098495,B=1.000000,A=1.000000)" 0.0 0.0)))))